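; Multi-floor lift that comes to the floor it is called from and carries the first-person character to a random floor.
; Construction stacks meshes and a BP_Call per floor, linked back through LiftRef, and randomizes the lift and player start floors.
; Join and the Detector overlap share one move, timed by floor distance, with timeline-driven sliding doors.
; The overlap's re-roll tests LiftFloor rather than GoTo, so it loops endlessly from floor 0.
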(event `Join`
  (params (WhereFrom :type Integer))
  (if (== WhereFrom (`self.LiftFloor`))
    (`self.OpenClose` false)
    (else
      (`self.OpenClose` true)
      (set `self.GoTo` WhereFrom)
      (`KismetSystemLibrary.MoveComponentTo` (`self.Lift`) (`KismetMathLibrary.MakeVector` 0.0 0.0 (`KismetMathLibrary.Conv_IntToDouble` (* (`self.GoTo`) 1000))) (struct) false false (* (`KismetMathLibrary.Abs` (- (`self.GoTo`) (`self.LiftFloor`))) 2.5) :!label _label)
      (set `self.LiftFloor` (`self.GoTo`))
      (`self.OpenClose` false))))

(event `self.Detector.OnComponentBeginOverlap`
  (params (OverlappedComponent :type "PrimitiveComponent Object Reference") (OtherActor :type "Actor Object Reference") (OtherComp :type "PrimitiveComponent Object Reference") (OtherBodyIndex :type Integer) (bFromSweep :type Boolean) (SweepResult :type "HitResult Structure (by ref)"))
  (cast `/Game/FirstPerson/Blueprints/BP_FirstPersonCharacter` OtherActor)
  (`self.OpenClose` true)
  (set `self.GoTo` (`KismetMathLibrary.RandomInteger` (`self.Number_Floors`)) :!label _label_2)
  (if (== (`self.LiftFloor`) 0)
    (goto _label_2)
    (else
      (`KismetSystemLibrary.Delay` 1.0)
      (goto _label))))

(event `OpenClose`
  (params (IsClosed :type Boolean))
  (`|ExecutionSequence`
    (:`then_0`
      (if IsClosed
        (bind (_direction _newtrack_0) (`Timeline|Timeline` :!via `ReverseFromEnd` :!label _label_3)
          (:`Update`
            (`SceneComponent.K2_SetRelativeLocation` (`self.SM_Lift01Door03`) (`KismetMathLibrary.MakeVector` (`KismetMathLibrary.Lerp` 0.0 -65.0 _newtrack_0) -55.0) false false)
            (`SceneComponent.K2_SetRelativeLocation` (`self.SM_Lift01Door01`) (`KismetMathLibrary.MakeVector` (`KismetMathLibrary.Lerp` 0.0 65.0 _newtrack_0)) false false)))
        (else
          (goto _label_3 :!via `PlayFromStart`))))))

(fn `UserConstructionScript`
  (`SceneComponent.K2_SetWorldLocation` (`Actor.RootComponent` (`self.PlayerStartRef`)) (`KismetMathLibrary.MakeVector` 1405.0 2250.0 (`KismetMathLibrary.Conv_IntToDouble` (+ (* (`KismetMathLibrary.RandomInteger` (`self.Number_Floors`)) 1000) 195))) false false)
  (bind _output_get (set `self.LiftFloor` (`KismetMathLibrary.RandomInteger` (`self.Number_Floors`))))
  (`SceneComponent.K2_SetRelativeLocation` (`self.Lift`) (`KismetMathLibrary.MakeVector` 0.0 0.0 (`KismetMathLibrary.Conv_IntToDouble` (* _output_get 1000))) false false)
  (for _index (range (+ (`self.Number_Floors`) 1))
    (bind _returnvalue (`KismetMathLibrary.Conv_IntToDouble` (* _index 1000)))
    (`AddComponent|NODE_AddStaticMeshComponent-0` :`RelativeTransform` (`KismetMathLibrary.MakeTransform` (`KismetMathLibrary.MakeVector` 0.0 520.0 _returnvalue)))
    (`AddComponent|NODE_AddStaticMeshComponent-1` :`RelativeTransform` (`KismetMathLibrary.MakeTransform` (`KismetMathLibrary.MakeVector` 0.0 0.0 _returnvalue)))
    (`AddComponent|NODE_AddStaticMeshComponent-3` :`RelativeTransform` (`KismetMathLibrary.MakeTransform` (`KismetMathLibrary.MakeVector` 0.0 0.0 (+ _returnvalue 500.0))))
    (bind _returnvalue_2 (`AddComponent|NODE_AddChildActorComponent-0` :`RelativeTransform` (`KismetMathLibrary.MakeTransform` (`KismetMathLibrary.MakeVector` -105.0 0.0 (+ _returnvalue 130.0)))))
    (bind _asbp_call (cast `/Game/Lift/Blueprint/BP_Call` (`ChildActorComponent.ChildActor` _returnvalue_2)))
    (set `/Game/Lift/Blueprint/BP_Call.IndexFloor` _index _asbp_call)
    (set `/Game/Lift/Blueprint/BP_Call.LiftRef` self _asbp_call)))